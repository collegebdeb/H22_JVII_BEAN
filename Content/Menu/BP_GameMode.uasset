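; Game mode that persists the player character's transform in a single save slot.
; On BeginPlay it creates the BP_SaveGame slot if missing, otherwise applies the saved transform to the ThirdPersonCharacter's mesh rather than the actor.
; SaveGame writes the character's actor transform into that slot.
; LoadGame reads no save data itself and only executes the "Partie" console command.
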(event Custom|SaveGame
  (bind _returnvalue (SaveGame|LoadGamefromSlot "save_1"))
  (bind _asbp_save_game (Utilities|Casting|CastToBP_SaveGame _returnvalue))
  (Variables|/Game/Menu/BP_SaveGame.BP_SaveGame_C|SetChar_Transform _asbp_save_game (Transformation|GetActorTransform (.AsThird%20Person%20Character (Utilities|Casting|CastToThirdPersonCharacter (Game|GetPlayerCharacter 0)))))
  (SaveGame|SaveGametoSlot _asbp_save_game "save_1"))

(event Custom|LoadGame
  (Development|ExecuteConsoleCommand "Partie" 0))

(event EventBeginPlay
  (bind _returnvalue (SaveGame|DoesSaveGameExist "save_1"))
  (if _returnvalue
    (bind _returnvalue_2 (SaveGame|LoadGamefromSlot "save_1"))
    (bind _asbp_save_game (Utilities|Casting|CastToBP_SaveGame _returnvalue_2))
    (bind _asthird_person_character (Utilities|Casting|CastToThirdPersonCharacter (Game|GetPlayerCharacter 0)))
    (Transformation|SetWorldTransform (Variables|/Script/Engine.Character|GetMesh _asthird_person_character) (Variables|/Game/Menu/BP_SaveGame.BP_SaveGame_C|GetChar_Transform _asbp_save_game) false false)
    (else
      (bind _returnvalue_3 (SaveGame|CreateSaveGameObject "/Game/Menu/BP_SaveGame.BP_SaveGame_C"))
      (SaveGame|SaveGametoSlot _returnvalue_3 "save_1"))))

(fn ConstructionScript)